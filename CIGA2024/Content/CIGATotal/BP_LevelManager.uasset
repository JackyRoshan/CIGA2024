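; BP_LevelManager is a level manager Blueprint that builds an ordered list of the food spawners in the level.
; On BeginPlay it gathers every BP_FoodSpawner actor into SpawnerArray.
; It then sorts the array in ascending SpawnerNum order with an in-place nested-loop exchange sort, so the order does not depend on how the actors are returned.
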(event EventBeginPlay
  (bind _outactors (Actor|GetAllActorsOfClass "/Game/CIGATotal/Item/BP_FoodSpawner.BP_FoodSpawner_C"))
  (bind _output_get (Variables|Default|SetSpawnerArray _outactors))
  (for _index (range 0 (Utilities|Array|LastIndex _output_get))
    (for _index_2 (range _index (Utilities|Array|LastIndex _output_get))
      (if (> (Variables|/Game/CIGATotal/Item/BP_FoodSpawner.BP_FoodSpawner_C|GetSpawnerNum (Utilities|Array|Get(acopy) _output_get _index)) (Variables|/Game/CIGATotal/Item/BP_FoodSpawner.BP_FoodSpawner_C|GetSpawnerNum (Utilities|Array|Get(acopy) _output_get _index_2)))
        (Utilities|Array|Swap _output_get _index_2 _index)))))

(fn ConstructionScript)