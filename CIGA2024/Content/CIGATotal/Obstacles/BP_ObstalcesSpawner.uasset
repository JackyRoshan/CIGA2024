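; Obstacle spawner actor that periodically drops a random obstacle at its location, preceded by a warning.
; A randomized timer fires RandomObstacles, which spawns BP_Warning at the spawner's X/Y and the player pawn's height.
; After a short delay it spawns a random class from MainGameMode's Obstacles list.
; Both the warning and obstacle steps reset the timer with the newly rolled interval.
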(event Custom|RandomObstacles
  (bind _returnvalue (Transformation|GetActorTransform))
  (bind _returnvalue_2 (Transformation|GetActorTransform))
  (bind _asmain_game_mode (Utilities|Casting|CastToMainGameMode (Game|GetGameMode)))
  (Variables|Default|SetRandomNum (Math|Random|RandomFloatinRange 8.0 12.0))
  (Utilities|FlowControl|Sequence
    (:then_0
      (Game|SpawnActorfromClass "/Game/CIGATotal/Others/BP_Warning.BP_Warning_C" (Math|Transform|MakeTransform (Math|Vector|MakeVector (.x (.location _returnvalue)) (.y (.location _returnvalue)) (.z (.location (Transformation|GetActorTransform (Game|Player|GetPlayerPawn 0))))) (.rotation _returnvalue) "1.000000,1.000000,1.000000") "Undefined" "MultiplyWithRoot" 0 0))
    (:then_1
      (Utilities|FlowControl|Delay 3.0)
      (Game|SpawnActorfromClass (.OutItem (Utilities|Array|Random (Variables|/Game/CIGATotal/MainGameMode.MainGameMode_C|GetObstacles _asmain_game_mode))) (Math|Transform|MakeTransform (.location _returnvalue_2) (.rotation _returnvalue_2) "1.000000,1.000000,1.000000") "Undefined" "MultiplyWithRoot" 0 0)))
  (Utilities|Time|ClearandInvalidateTimerbyHandle (Variables|Default|GetTimerHandle))
  (CallFunction|Timer))

(event Custom|Timer
  (bind _returnvalue (Utilities|Time|SetTimerbyEvent (delegate Custom|RandomObstacles) (Variables|Default|GetRandomNum) true))
  (Variables|Default|SetTimerHandle _returnvalue))

(event EventBeginPlay
  (Variables|Default|SetRandomNum (Math|Random|RandomFloatinRange 9.0 15.0))
  (bind _returnvalue (Utilities|Time|SetTimerbyEvent (delegate Custom|RandomObstacles) (Variables|Default|GetRandomNum) true))
  (Variables|Default|SetTimerHandle _returnvalue))

(fn ConstructionScript)