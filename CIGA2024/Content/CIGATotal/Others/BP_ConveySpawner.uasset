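; Conveyor spawner that periodically spawns a random obstacle (cup, water or plate) at its own transform.
; On BeginPlay it converts its Direction enum into a positive or negative multiplier and starts a looping timer.
; The timer's negative initial delay offsets the interval, so the first spawn happens almost immediately.
; Each spawned obstacle receives the direction multiplier.
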(event Custom|RandomObstacles
  (bind _returnvalue (Transformation|GetActorTransform))
  (bind _returnvalue_2 (Transformation|GetActorTransform))
  (bind _returnvalue_3 (Transformation|GetActorTransform))
  (switch int (Math|Random|RandomIntegerinRange 0 2)
    (:0
      (Game|SpawnActorfromClass "/Game/CIGATotal/Others/Cup.Cup_C" (Math|Transform|MakeTransform (.location _returnvalue) (.rotation _returnvalue) "1.000000,1.000000,1.000000") "Undefined" "MultiplyWithRoot" 0 (Variables|Default|GetDirectMuti) 0))
    (:1
      (Game|SpawnActorfromClass "/Game/CIGATotal/Others/Water.Water_C" (Math|Transform|MakeTransform (.location _returnvalue_2) (.rotation _returnvalue_2) "1.000000,1.000000,1.000000") "Undefined" "MultiplyWithRoot" 0 (Variables|Default|GetDirectMuti) 0))
    (:2
      (Game|SpawnActorfromClass "/Game/CIGATotal/Others/Plate.Plate_C" (Math|Transform|MakeTransform (.location _returnvalue_3) (.rotation _returnvalue_3) "1.000000,1.000000,1.000000") "Undefined" "MultiplyWithRoot" 0 (Variables|Default|GetDirectMuti) 0))))

(event EventBeginPlay
  (if (Utilities|Enum|Equal(Enum) (Variables|Default|GetDirection) "NewEnumerator1")
    (Variables|Default|SetDirectMuti 1.0)
    (else
      (Variables|Default|SetDirectMuti -1.0)))
  (bind _returnvalue (Utilities|Time|SetTimerbyEvent (delegate Custom|RandomObstacles) 1e+01 true -1e+01))
  (Variables|Default|SetSpawnerTimer _returnvalue))

(event Collision|EventActorBeginOverlap
  (params (OtherActor :type Actor%20Object%20Reference)))

(event EventTick
  (params (DeltaSeconds :type Float%20%28single-precision%29)))

(fn ConstructionScript)