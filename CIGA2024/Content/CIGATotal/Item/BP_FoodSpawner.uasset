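; BP_FoodSpawner is a food spawner that creates a randomly chosen food item at its own transform.
; A looping timer, offset to fire almost immediately from BeginPlay, rolls a food index and calls FoodSelect to spawn ItemBase.
; Each item receives the spawner number and food index through MatchNumMessage.
; GetFood clears the timer and restarts it after a short delay, triggering a fresh spawn.
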(event Custom|RandomFood
  (Variables|Default|SetFoodNum (Math|Random|RandomIntegerinRange 0 7))
  (Utilities|FoodSelect "/Game/CIGATotal/Item/ItemBase.ItemBase_C"))

(event EventBeginPlay
  (bind _returnvalue (Utilities|Time|SetTimerbyEvent (delegate Custom|RandomFood) 1e+01 true -1e+01))
  (Variables|Default|SetSpawnerTimer _returnvalue))

(event EventGetFood
  (Utilities|Time|ClearandInvalidateTimerbyHandle (Variables|Default|GetSpawnerTimer))
  (Utilities|FlowControl|Delay 3.0)
  (bind _returnvalue (Utilities|Time|SetTimerbyEvent (delegate Custom|RandomFood) 1e+01 true -1e+01))
  (Variables|Default|SetSpawnerTimer _returnvalue))

(fn ConstructionScript)