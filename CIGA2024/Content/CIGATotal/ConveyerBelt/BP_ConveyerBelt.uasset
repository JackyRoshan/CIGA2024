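; Conveyor belt actor that scrolls left or right and tells obstacles entering its trigger box which way to turn.
; A looping timer steps two belt components along X by speed and step length, wrapping each to the opposite end for an endless loop.
; For left-to-right, both belts are rotated 180 degrees at BeginPlay.
; Box overlap flags ObstacleBase actors as landed and sets TurnLeft from the belt direction.
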(event OnComponentBeginOverlap(Box)
  (params (OverlappedComponent :type Primitive%20Component%20Object%20Reference) (OtherActor :type Actor%20Object%20Reference) (OtherComp :type Primitive%20Component%20Object%20Reference) (OtherBodyIndex :type Integer) (bFromSweep :type Boolean) (SweepResult :type Hit%20Result%20Structure%20%28by%20ref%29))
  (bind _asobstacle_base (Utilities|Casting|CastToObstacleBase OtherActor))
  (Variables|/Game/CIGATotal/Obstacles/ObstacleBase.ObstacleBase_C|SetLand? _asobstacle_base true)
  (if (Utilities|Enum|Equal(Enum) (Variables|Default|GetDirection) "NewEnumerator0")
    (Variables|/Game/CIGATotal/Obstacles/ObstacleBase.ObstacleBase_C|SetTurnLeft? _asobstacle_base true)
    (else
      (Variables|/Game/CIGATotal/Obstacles/ObstacleBase.ObstacleBase_C|SetTurnLeft? _asobstacle_base false))))

(event Custom|MoveConveyer
  (bind _belt1 (Variables|Default|GetBelt1))
  (bind _belt2 (Variables|Default|GetBelt2))
  (bind _belt2_2 (Variables|Default|GetBelt2))
  (bind _belt1_2 (Variables|Default|GetBelt1))
  (switch Utilities|FlowControl|Switch|SwitchonConveyDirection (Variables|Default|GetDirection)
    (:NewEnumerator0
      (Utilities|FlowControl|Sequence
        (:then_0
          (Transformation|AddRelativeLocation (Variables|Default|GetBelt1) (Math|Vector|MakeVector (* (* (Variables|Default|GetSpeed) (Variables|Default|GetMoveStepLength)) -1.0) 0.0 0.0) false false))
        (:then_1
          (Transformation|AddRelativeLocation (Variables|Default|GetBelt2) (Math|Vector|MakeVector (* (* (Variables|Default|GetSpeed) (Variables|Default|GetMoveStepLength)) -1.0) 0.0 0.0) false false))
        (:then_2
          (if (<= (.x (Variables|/Script/Engine.SceneComponent|GetRelativeLocation _belt1_2)) -2.4e+03)
            (Transformation|SetRelativeLocation _belt1_2 "2400.000000,0.000000,0.000000" false false)))
        (:then_3
          (if (<= (.x (Variables|/Script/Engine.SceneComponent|GetRelativeLocation _belt2_2)) -2.4e+03)
            (Transformation|SetRelativeLocation _belt2_2 "2400.000000,0.000000,0.000000" false false)))))
    (:NewEnumerator1
      (Utilities|FlowControl|Sequence
        (:then_0
          (Transformation|AddRelativeLocation (Variables|Default|GetBelt1) (Math|Vector|MakeVector (* (Variables|Default|GetSpeed) (Variables|Default|GetMoveStepLength)) 0.0 0.0) false false))
        (:then_1
          (Transformation|AddRelativeLocation (Variables|Default|GetBelt2) (Math|Vector|MakeVector (* (Variables|Default|GetSpeed) (Variables|Default|GetMoveStepLength)) 0.0 0.0) false false))
        (:then_2
          (if (>= (.x (Variables|/Script/Engine.SceneComponent|GetRelativeLocation _belt1)) 2.4e+03)
            (Transformation|SetRelativeLocation _belt1 "-2400.000000,0.000000,0.000000" false false)))
        (:then_3
          (if (>= (.x (Variables|/Script/Engine.SceneComponent|GetRelativeLocation _belt2)) 2.4e+03)
            (Transformation|SetRelativeLocation _belt2 "-2400.000000,0.000000,0.000000" false false)))))))

(event EventBeginPlay
  (Utilities|FlowControl|Sequence
    (:then_0
      (switch Utilities|FlowControl|Switch|SwitchonConveyDirection (Variables|Default|GetDirection)
        (:NewEnumerator1
          (Transformation|AddRelativeRotation (Variables|Default|GetBelt1) "0.000000,180.000000,0.000000" false false)
          (Transformation|AddRelativeRotation (Variables|Default|GetBelt2) "0.000000,180.000000,0.000000" false false))))
    (:then_1
      (Utilities|Time|SetTimerbyEvent (delegate Custom|MoveConveyer) 0.04 true))))

(event Collision|EventActorBeginOverlap
  (params (OtherActor :type Actor%20Object%20Reference)))

(event EventTick
  (params (DeltaSeconds :type Float%20%28single-precision%29)))

(fn ConstructionScript)